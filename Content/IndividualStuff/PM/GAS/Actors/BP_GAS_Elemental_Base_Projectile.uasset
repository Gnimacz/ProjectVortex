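; Base GAS elemental projectile that applies gameplay effects to characters it hits or overlaps, skipping its owner on overlap.
; Construction sets optional homing and aims at a given target, the owning player's target, or the camera direction.
; Effect tags are matched to damage table rows for SetByCaller magnitudes, with specs made and applied by the victim's own ASC.
; Impact spawns particles, optionally ground-traced on overlap, then destroys the projectile.
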(event `self.ReceiveHit`
  (params (MyComp :type "PrimitiveComponent Object Reference") (Other :type "Actor Object Reference") (OtherComp :type "PrimitiveComponent Object Reference") (bSelfMoved :type Boolean) (HitLocation :type "Vector Structure") (HitNormal :type "Vector Structure") (NormalImpulse :type "Vector Structure") (Hit :type "HitResult Structure (by ref)"))
  (bind _returnvalue (`self.K2_GetActorLocation`))
  (set `self.Place At Feet?` false)
  (set `self.HitActor` Other)
  (bind _ascharacter (cast `Character` (`self.HitActor`) :!label _label)
    (:`then`
      (`self.Apply Gameplay Effect to Hit Actor` _ascharacter))
    (:`CastFailed`
      _))
  (if (`self.Place At Feet?`)
    (bind (_outhit _returnvalue_2) (`KismetSystemLibrary.LineTraceSingleForObjects` :`Start` _returnvalue :`End` (+ _returnvalue (0.0 0.0 -500.0)) :`ObjectTypes` (`|MakeArray` "ObjectTypeQuery1" "ObjectTypeQuery2" :!type "EObjectTypeQuery Enum") :`DrawDebugType` "ForDuration")))
  (`GameplayStatics.SpawnEmitterAtLocation` (`self.ProjectileHitParticle`) (`KismetMathLibrary.SelectVector` (`.ImpactPoint` (`GameplayStatics.BreakHitResult` _outhit)) (+ (`KismetMathLibrary.SelectVector` HitLocation (`self.K2_GetActorLocation` (stale `self.ReceiveActorBeginOverlap` _output_get)) (`KismetSystemLibrary.IsValid` Other)) (`self.Hit Particle Offset`)) (and _returnvalue_2 (`self.Place At Feet?`))) (`KismetMathLibrary.SelectRotator` (`KismetMathLibrary.MakeRotFromZ` HitNormal) (struct) (`self.ShouldFaceSurface?`)))
  (`self.K2_DestroyActor`))

(event `self.ReceiveActorBeginOverlap`
  (params (OtherActor :type "Actor Object Reference"))
  (bind _ascharacter (cast `Character` OtherActor))
  (bind _output_get (set `self.HitActor` _ascharacter))
  (if (not (== _output_get (`self.GetOwner`)))
    (goto _label)))

(fn `Apply Gameplay Effect to Hit Actor`
  (params (Actor :type "Actor Object Reference"))
  (locals (FoundName :type Boolean))
  (bind _returnvalue (`AbilitySystemBlueprintLibrary.GetAbilitySystemComponent` Actor))
  (bind _effects_to_apply (`self.Effects To Apply`))
  (`/Engine/EditorBlueprintResources/StandardMacros.IsValid` _returnvalue
    (:`Is Valid`
      (bind _values (`BlueprintMapLibrary.Map_Values` _effects_to_apply))
      (for (_array_element _array_index) _values
        (for _array_element_2 (`BlueprintGameplayTagLibrary.BreakGameplayTagContainer` _array_element)
          (bind _keys (`BlueprintMapLibrary.Map_Keys` _effects_to_apply))
          (bind _outrownames (`DataTableFunctionLibrary.GetDataTableRowNames` "/Game/IndividualStuff/Cat/DataTables/Damage_Values.Damage_Values"))
          (for _array_element_3 _outrownames
            (bind _returnvalue_2 (`|GetDataTableRow` "/Game/IndividualStuff/Cat/DataTables/Damage_Values.Damage_Values" _array_element_3)
              (:`then`
                (bind (_skill_id _skill_name _skill_dmg) (break `/Game/IndividualStuff/Cat/DataTables/PlayerAbilitiesStruct` _returnvalue_2))
                (if (== _skill_name (`KismetStringLibrary.Conv_NameToString` (`BlueprintGameplayTagLibrary.GetTagName` _array_element_2)))
                  (bind _returnvalue_3 (`AbilitySystemBlueprintLibrary.AssignTagSetByCallerMagnitude` (`AbilitySystemComponent.MakeOutgoingSpec` _returnvalue (`|GetArrayItem` _keys _array_index) 0.0 (`AbilitySystemComponent.MakeEffectContext` _returnvalue)) (struct) (`KismetMathLibrary.Conv_IntToDouble` _skill_dmg)))
                  (`AbilitySystemComponent.BP_ApplyGameplayEffectSpecToTarget` _returnvalue _returnvalue_3 _returnvalue))))))))))

(fn `Find Name From Tag`
  (params (String :type String))
  (returns (Name :type String))
  (locals (FoundName :type Boolean) (Name :type String))
  (return (`.RightS` (`KismetStringLibrary.Split` String "." "IgnoreCase" "FromEnd"))))

(fn `Set Value in Gameplay Effect`
  (params (`Data Tag` :type "Array of GameplayTag Structure") (`Effect Level` :type "Float (single-precision)") (Magnitude :type "Float (single-precision)"))
  (set `self.Damage Tag` `Data Tag`)
  (set `self.Effect Level` `Effect Level`)
  (set `self.Magnitude` Magnitude))

(fn `UserConstructionScript`
  (set `ProjectileMovementComponent.InitialSpeed` (`self.ProjectileSpeed`) (`self.ProjectileMovement`))
  (`ParticleSystemComponent.SetTemplate` (`self.ParticleSystem`) (`self.ProjectileParticle`))
  (bind _output_get (set `ProjectileMovementComponent.bIsHomingProjectile` (`self.Homing?`) (`self.ProjectileMovement`)))
  (if _output_get
    (`/Engine/EditorBlueprintResources/StandardMacros.IsValid` (`self.Target`)
      (:`Is Valid`
        (bind _ascharacter (cast `Character` (`self.Target`))
          (:`then`
            (set `ProjectileMovementComponent.HomingTargetComponent` (`Character.CapsuleComponent` _ascharacter) (`self.ProjectileMovement`))
            (set `ProjectileMovementComponent.HomingAccelerationMagnitude` (`self.Homing Speed`) (`self.ProjectileMovement`))
            (`self.K2_SetActorRotation` (`KismetMathLibrary.FindLookAtRotation` (`self.K2_GetActorLocation`) (`self.K2_GetActorLocation` (`self.Target`))) true :!label _label))
          (:`CastFailed`
            (bind _asbp_gas_player_character_base (cast `/Game/IndividualStuff/PM/GAS/Characters/Player/BP_GAS_PlayerCharacter_Base` (`self.GetOwner`) :!label _label_2))
            (`self.K2_SetActorRotation` (`KismetMathLibrary.Conv_VectorToRotator` (`SceneComponent.GetForwardVector` (`/Game/IndividualStuff/PM/GAS/Characters/Player/BP_GAS_PlayerCharacter_Base.FollowCamera` _asbp_gas_player_character_base))) true))))
      (:`Is Not Valid`
        (bind _asbp_gas_player_character_base_2 (cast `/Game/IndividualStuff/PM/GAS/Characters/Player/BP_GAS_PlayerCharacter_Base` (`self.GetOwner`) :!label _label_3))
        (bind _selectedtarget (`/Game/IndividualStuff/PM/GAS/Characters/Player/BP_GAS_PlayerCharacter_Base.Get Target` _asbp_gas_player_character_base_2))
        (`/Engine/EditorBlueprintResources/StandardMacros.IsValid` _selectedtarget
          (:`Is Valid`
            (bind _ascharacter_2 (cast `Character` _selectedtarget)
              (:`then`
                (set `self.Target` _ascharacter_2)
                (set `ProjectileMovementComponent.HomingTargetComponent` (`Character.CapsuleComponent` _ascharacter_2) (`self.ProjectileMovement`))
                (goto _label))
              (:`CastFailed`
                (goto _label_2))))
          (:`Is Not Valid`
            (goto _label_2)))))
    (else
      (goto _label_3))))