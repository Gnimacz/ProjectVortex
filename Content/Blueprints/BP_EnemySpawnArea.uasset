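; Enemy spawn area that runs configured enemy waves, armed by its first actor overlap.
; Each wave builds a shuffled queue from its class-to-count map, then spawns enemies at random spawn points after a brief effect, spaced by wave delays.
; Tick launches the next wave once the EnemyManager's alive count drops to its trigger threshold.
; A looping timer, started only if that first overlap is the player, flags a random ready enemy to attack.
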(event `self.ReceiveBeginPlay`
  (set `self.Started` false))

(event `self.ReceiveActorBeginOverlap`
  (params (OtherActor :type "Actor Object Reference"))
  (if (not (`self.Started`))
    (set `self.Started` true)
    (if (== OtherActor (`GameplayStatics.GetPlayerPawn` 0))
      (if (> (`KismetArrayLibrary.Array_Length` (`self.Waves`)) 0)
        (`KismetSystemLibrary.PrintText` "Starting waves")
        (`KismetSystemLibrary.K2_SetTimer` null "MakeEnemyAttack" 5.0 true)
        (`self.SpawnWave_Event` 0)
        (else
          (`KismetSystemLibrary.PrintText` "There are no waves defined in this spawn area" true true (struct :`R` 1.0 :`A` 1.0)))))))

(event `SpawnWave_Event`
  (params (Index :type Integer))
  (bind _waves (`self.Waves`))
  (set `self.WaveOngoing` true)
  (if (< Index (`KismetArrayLibrary.Array_Length` _waves))
    (`self.FillSpawnQueue`)
    (`KismetSystemLibrary.Delay` (`.Delay_2_11ED1CDE44FF53062ADC3C889A3B54D1` (break `/Game/Blueprints/Wave` (`|GetArrayItem` _waves Index))))
    (`self.SpawnEnemy_Event` :!label _label)))

(event `SpawnEnemy_Event`
  (bind _queue (`self.Queue`))
  (bind _spawnpoints (`self.SpawnPoints`))
  (if (> (`KismetArrayLibrary.Array_Length` (`self.Queue`)) 0)
    (if (> (`KismetArrayLibrary.Array_Length` _spawnpoints) 0)
      ;[1 1 1] Create spawn effect and wait for its animation
      (bind _returnvalue (`|SpawnActorFromClass` "/Game/Blueprints/BP_EnemySpawnEffect.BP_EnemySpawnEffect_C" (`self.GetTransform` (`KismetArrayLibrary.Array_Random` _spawnpoints)) "AlwaysSpawn" "MultiplyWithRoot" null null))
      (`KismetSystemLibrary.Delay` 0.5)
      (`|SpawnActorFromClass` (`|GetArrayItem` (`self.Queue`)) (`KismetMathLibrary.MakeTransform` (+ (.location (`self.GetTransform` _returnvalue)) (0.0 0.0 85.0))) "Undefined" "MultiplyWithRoot" null null)
      (`KismetArrayLibrary.Array_Remove` _queue)
      (if (> (`KismetArrayLibrary.Array_Length` _queue) 0)
        (`KismetSystemLibrary.Delay` (`.TimeBetweenSpawns_4_8F7B8130488FF1722102F7BFB11F37EE` (break `/Game/Blueprints/Wave` (`|GetArrayItem` (`self.Waves`) (stale `SpawnWave_Event` Index)))))
        (goto _label)
        (else
          (set `self.WaveOngoing` false)
          (set `self.CurrentWaveIndex` (+ (`self.CurrentWaveIndex`) 1))))
      (else
        (`KismetSystemLibrary.PrintText` "There are no spawn points defined for this area!" true true (struct :`R` 1.0 :`A` 1.0))))
    (else
      (`KismetSystemLibrary.PrintText` "There are no enemies in this wave!" true true (struct :`R` 1.0 :`G` 0.016463 :`A` 1.0)))))

(event `self.ReceiveTick`
  (params (DeltaSeconds :type "Float (single-precision)"))
  (if (`self.Started`)
    (if (`self.WaveOngoing`)
      _
      (elif (< (`self.CurrentWaveIndex`) (`KismetArrayLibrary.Array_Length` (`self.Waves`)))
        (bind _ascustom_game_instance (cast `/Game/Blueprints/CustomGameInstance` (`GameplayStatics.GetGameInstance`)))
        (if (<= (`KismetArrayLibrary.Array_Length` (`/Game/Blueprints/BP_AliveEnemiesManager.AliveEnemies` (`/Game/Blueprints/CustomGameInstance.EnemyManager` _ascustom_game_instance))) (`.TriggerCondition_7_9C5F4590407F70E5FD0882BA61326C98` (break `/Game/Blueprints/Wave` (`|GetArrayItem` (`self.Waves`) (`self.CurrentWaveIndex`)))))
          (`self.SpawnWave_Event` (`self.CurrentWaveIndex`)))))))

(fn `FillSpawnQueue`
  (bind (_delay _timebetweenspawns _triggercondition _enemies) (break `/Game/Blueprints/Wave` (`|GetArrayItem` (`self.Waves`) (`self.CurrentWaveIndex`))))
  (`KismetArrayLibrary.Array_Clear` (`self.Queue`))
  (bind _keys (`BlueprintMapLibrary.Map_Keys` _enemies))
  (for _array_element _keys
    (for _ (range 1 (+ (`BlueprintMapLibrary.Map_Find` _enemies _array_element) 1))
      (`KismetArrayLibrary.Array_Add` (`self.Queue`) _array_element)))
  (`KismetArrayLibrary.Array_Shuffle` (`self.Queue`)))

(fn `MakeEnemyAttack`
  (locals (ReadyToAttackList :type "Array of /Game/Blueprints/Enemies/BP_EnemyBase Object Reference"))
  (bind _readytoattacklist (`local.ReadyToAttackList`))
  (bind _ascustom_game_instance (cast `/Game/Blueprints/CustomGameInstance` (`GameplayStatics.GetGameInstance`)))
  (`KismetArrayLibrary.Array_Clear` (`local.ReadyToAttackList`))
  (bind _aliveenemies (`/Game/Blueprints/BP_AliveEnemiesManager.AliveEnemies` (`/Game/Blueprints/CustomGameInstance.EnemyManager` _ascustom_game_instance)))
  (if (> (`KismetArrayLibrary.Array_Length` _aliveenemies) 0)
    (for _array_element _aliveenemies
      (if (`/Game/Blueprints/Enemies/BP_EnemyBase.ReadyToAttack` _array_element)
        (`KismetArrayLibrary.Array_Add` (`local.ReadyToAttackList`) _array_element)))
    (if (> (`KismetArrayLibrary.Array_Length` _readytoattacklist) 0)
      (set `/Game/Blueprints/Enemies/BP_EnemyBase.ShouldAttack` true (`KismetArrayLibrary.Array_Random` _readytoattacklist)))))

(fn `UserConstructionScript`)